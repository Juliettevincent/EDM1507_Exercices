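; MIDI manager Blueprint that plays a polyphonic MetaSound synth from an external MIDI controller.
; BeginPlay opens the input device matching MIDIControlerIndex and binds its MIDI events.
; Note On spawns a PolySynth sound stored in PolyVoices by note number, Note Off triggers its release, and CC 71 sets Amount on all voices.
; A MonoSynth is also created, but its playback and CC mappings are disconnected.
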(event Custom|EventOnMidiEvent
  (params (MIDIDeviceController :type MIDI%20Device%20Controller%20Object%20Reference) (Timestamp :type Integer) (EventType :type EMIDIEventType%20Enum :default "Unknown") (Channel :type Integer) (ControlID :type Integer) (Velocity :type Integer) (RawEventType :type Integer))
  (bind _returnvalue (Math|Conversions|ToFloat(Integer) ControlID))
  (bind _returnvalue_2 (Math|Float|Truncate _returnvalue))
  (Development|PrintString (Utilities|String|ToString(Text) (Utilities|Text|FormatText "MIDI Note {note} VELOCITY {velocity} MIDI EVENT TYPE {event}" ControlID Velocity (Utilities|String|EnumtoString EventType))) true true "(R=1.000000,G=0.214506,B=0.040962,A=1.000000)" 2.0 "MIDI")
  (switch Utilities|FlowControl|Switch|SwitchonEMIDIEventType EventType
    (:NoteOff
      (Class|AudioParameterControllerInterface|SetTriggerParameter (Utilities|Array|Get(acopy) (Variables|Default|GetPolyVoices) _returnvalue_2) "Trigger Release"))
    (:NoteOn
      (bind _returnvalue_3 (Audio|CreateSound2D "/Game/MetaSound/MSS_PolySynth.MSS_PolySynth" 1.0 1.0 0.0 0))
      (Utilities|Array|SetArrayElem (Variables|Default|GetPolyVoices) _returnvalue_2 _returnvalue_3 true)
      (Audio|Parameter|SetFloatParameter _returnvalue_3 "MIDI Note" _returnvalue :!class /Script/AudioExtensions.AudioParameterControllerInterface)
      (Audio|Components|Audio|Play _returnvalue_3 0.0))
    (:ControlChange
      (switch string (Utilities|String|ToString(Integer) _returnvalue_2)
        (:71
          (for _array_element (Variables|Default|GetPolyVoices)
            (Utilities|IsValid _array_element
              (:Is%20Valid
                (Audio|Parameter|SetFloatParameter _array_element "Amount" (/ (Math|Conversions|ToFloat(Integer) Velocity) 127.0) :!class /Script/AudioExtensions.AudioParameterControllerInterface)))))))))

(event EventBeginPlay
  (bind _outmididevices (Class|MIDIDeviceManager|FindMIDIDevices))
  (for _array_element _outmididevices
    (if (.bCanReceiveFrom (Utilities|Struct|BreakFoundMIDIDevice _array_element))
      (if (== (Variables|Default|GetMIDIControlerIndex) (.DeviceID (Utilities|Struct|BreakFoundMIDIDevice _array_element)))
        (Development|PrintString (.DeviceName (Utilities|Struct|BreakFoundMIDIDevice _array_element)))
        (bind _returnvalue (Class|MIDIDeviceManager|CreateMIDIDeviceController (.DeviceID (Utilities|Struct|BreakFoundMIDIDevice _array_element)) 1024))
        (bind _output_get (Variables|Default|SetNewVar _returnvalue))
        (EventDispatchers|BindEventtoOnMIDIEvent _output_get (EventDispatchers|CreateEvent :!event Custom|EventOnMidiEvent)))))
  (Development|PrintString "end for loop")
  (bind _returnvalue_2 (Audio|CreateSound2D "/Game/MetaSound/MSS_MonoSynth.MSS_MonoSynth" 1.0 1.0 0.0 0))
  (bind _output_get_2 (Variables|Default|SetMonoSynth _returnvalue_2)))

(fn ConstructionScript)